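; BP_Pickup is a spinning pickup actor that notifies its spawner when it is destroyed.
; It becomes collectable after a brief delay from BeginPlay, and Tick rotates its root by a fixed step each frame, independent of delta time.
; Its Destroy event searches all BP_PickupSpawner actors, calls Respawn on any whose ActorID matches SpawnID, then removes the pickup.
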(event Custom|Destroy
  (bind _outactors (Actor|GetAllActorsOfClass "/Game/Blueprints/BP_PickupSpawner.BP_PickupSpawner_C"))
  (for _array_element _outactors
    (if (== (Variables|/Game/Blueprints/BP_PickupSpawner.BP_PickupSpawner_C|GetActor%20ID _array_element) (Variables|Default|GetSpawnID))
      (Default|Respawn _array_element)))
  (Actor|DestroyActor))

(event EventBeginPlay
  (Utilities|FlowControl|Delay 0.2)
  (Variables|Default|SetCanCollect? true))

(event EventTick
  (params (DeltaSeconds :type Float%20%28single-precision%29))
  (Transformation|AddLocalRotation (Variables|Default|GetDefaultSceneRoot) "0,1.000000, 0" false false))

(fn ConstructionScript)