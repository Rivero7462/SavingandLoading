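; Game instance that holds player stats, level name and pickup spawn state, and saves, loads or deletes them through MySaveGame slots.
; Save reuses or creates the slot's save object; loading a missing slot copies a fresh object's defaults into the instance.
; Spawn records a unique ID and triggers the matching BP_PickupSpawner, while RemoveSpawn drops the ID and destroys matching BP_Pickup actors.
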(event Custom|SaveGame
  ;[0 0 0] SAVE LOAD DELETE
  ;;[1 0.4331 0.6261] Save List of Spawn Actors
  (bind _returnvalue (SaveGame|DoesSaveGameExist (Variables|Default|GetSaveSlot)))
  (if _returnvalue
    (bind _returnvalue_2 (SaveGame|LoadGamefromSlot (Variables|Default|GetSaveSlot)))
    (bind _asmy_save_game (Utilities|Casting|CastToMySaveGame _returnvalue_2))
    (Variables|Default|SetSave%20Game%20Ref _asmy_save_game)
    (else
      (bind _returnvalue_3 (SaveGame|CreateSaveGameObject "/Game/Blueprints/MySaveGame.MySaveGame_C"))
      (Variables|Default|SetSave%20Game%20Ref _returnvalue_3)))
  (Variables|/Game/Blueprints/MySaveGame.MySaveGame_C|SetSpawnActors (Variables|Default|GetSave%20Game%20Ref) (Variables|SavedData|GetSpawnID))
  (Variables|/Game/Blueprints/MySaveGame.MySaveGame_C|SetSpawnType (Variables|Default|GetSave%20Game%20Ref) (Variables|SavedData|GetSpawnType))
  (Variables|/Game/Blueprints/MySaveGame.MySaveGame_C|SetLevel%20Name (Variables|Default|GetSave%20Game%20Ref) (Variables|SavedData|GetLevel%20Name))
  (Variables|/Game/Blueprints/MySaveGame.MySaveGame_C|SetPlayerName (Variables|Default|GetSave%20Game%20Ref) (Variables|SavedData|GetPlayerName))
  (Variables|/Game/Blueprints/MySaveGame.MySaveGame_C|SetHealth (Variables|Default|GetSave%20Game%20Ref) (Variables|SavedData|GetHealth))
  (Variables|/Game/Blueprints/MySaveGame.MySaveGame_C|SetMagic (Variables|Default|GetSave%20Game%20Ref) (Variables|SavedData|GetMagic))
  (Variables|/Game/Blueprints/MySaveGame.MySaveGame_C|SetAmmo (Variables|Default|GetSave%20Game%20Ref) (Variables|SavedData|GetAmmo))
  (SaveGame|SaveGametoSlot (Variables|Default|GetSave%20Game%20Ref) (Variables|Default|GetSaveSlot)))

(event Custom|LoadGame
  (params (SlotName :type String))
  ;[0 0 0] SAVE LOAD DELETE
  ;;[0.4423 0.6952 1] Load list of Nonspawn Actors
  (bind _returnvalue (SaveGame|LoadGamefromSlot SlotName))
  (Utilities|IsValid _returnvalue
    (:Is%20Valid
      (bind _asmy_save_game (Utilities|Casting|CastToMySaveGame _returnvalue))
      (Variables|Default|SetSave%20Game%20Ref _asmy_save_game))
    (:Is%20Not%20Valid
      (bind _returnvalue_2 (SaveGame|CreateSaveGameObject "/Game/Blueprints/MySaveGame.MySaveGame_C"))
      (Variables|Default|SetSave%20Game%20Ref _returnvalue_2)))
  (Variables|SavedData|SetSpawnID (Variables|/Game/Blueprints/MySaveGame.MySaveGame_C|GetSpawnActors (Variables|Default|GetSave%20Game%20Ref)))
  (Variables|SavedData|SetSpawnType (Variables|/Game/Blueprints/MySaveGame.MySaveGame_C|GetSpawnType (Variables|Default|GetSave%20Game%20Ref)))
  (Variables|SavedData|SetLevel%20Name (Variables|/Game/Blueprints/MySaveGame.MySaveGame_C|GetLevel%20Name (Variables|Default|GetSave%20Game%20Ref)))
  (Variables|SavedData|SetPlayerName (Variables|/Game/Blueprints/MySaveGame.MySaveGame_C|GetPlayerName (Variables|Default|GetSave%20Game%20Ref)))
  (Variables|SavedData|SetHealth (Variables|/Game/Blueprints/MySaveGame.MySaveGame_C|GetHealth (Variables|Default|GetSave%20Game%20Ref)))
  (Variables|SavedData|SetMagic (Variables|/Game/Blueprints/MySaveGame.MySaveGame_C|GetMagic (Variables|Default|GetSave%20Game%20Ref)))
  (Variables|SavedData|SetAmmo (Variables|/Game/Blueprints/MySaveGame.MySaveGame_C|GetAmmo (Variables|Default|GetSave%20Game%20Ref))))

(event Custom|DeleteGame
  ;[0 0 0] SAVE LOAD DELETE
  ;;[0 0 0] Delete Game
  (SaveGame|DeleteGameinSlot (Variables|Default|GetSaveSlot)))

(event Custom|Spawn
  (params (SpawnID :type Integer%20%28by%20ref%29))
  (Utilities|Array|AddUnique (Variables|SavedData|GetSpawnID) SpawnID)
  ;[1 1 1] Do Within Level
  (bind _spawn (CallFunction|CheckifCanSpawn SpawnID))
  (if _spawn
    (bind _outactors (Actor|GetAllActorsOfClass "/Game/Blueprints/BP_PickupSpawner.BP_PickupSpawner_C"))
    (for _array_element _outactors
      (if (== (Variables|/Game/Blueprints/BP_PickupSpawner.BP_PickupSpawner_C|GetActor%20ID _array_element) SpawnID)
        (Default|SpawnNow _array_element)))))

(event Custom|RemoveSpawn
  (params (SpawnID :type Integer%20%28by%20ref%29))
  (Utilities|Array|RemoveItem (Variables|SavedData|GetSpawnID) SpawnID)
  ;[1 1 1] Do Within Level
  (bind _outactors (Actor|GetAllActorsOfClass "/Game/Blueprints/BP_Pickup.BP_Pickup_C"))
  (for _array_element _outactors
    (if (== (Variables|/Game/Blueprints/BP_Pickup.BP_Pickup_C|GetSpawnID _array_element) SpawnID)
      (Actor|DestroyActor _array_element))))

(event Custom|GetLevel
  (bind _returnvalue (Game|GetCurrentLevelName true))
  (Variables|SavedData|SetLevel%20Name (Utilities|String|StringToName _returnvalue)))

(fn CheckifCanSpawn
  (params (ItemID :type Integer%20%28by%20ref%29))
  (return (> (Utilities|Array|FindItem (Variables|SavedData|GetSpawnID) ItemID) -1)))