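; BP_Changes is a one-shot trigger actor that adds or removes spawn IDs in the game when the player character touches it.
; On BeginPlay, it builds a label from the AddRemove flag and the SpawnID list and shows it on a TextRender.
; When BP_ThirdPersonCharacter overlaps the Box, it calls Spawn or RemoveSpawn on MyGameInstance for each ID, then destroys itself.
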(event OnComponentBeginOverlap(Box)
  (params (OverlappedComponent :type Primitive%20Component%20Object%20Reference) (OtherActor :type Actor%20Object%20Reference) (OtherComp :type Primitive%20Component%20Object%20Reference) (OtherBodyIndex :type Integer) (bFromSweep :type Boolean) (SweepResult :type Hit%20Result%20Structure%20%28by%20ref%29))
  ;[1 1 1] Adds or Removes Spawn
  (Utilities|Casting|CastToBP_ThirdPersonCharacter OtherActor)
  (for _array_element (Variables|Default|GetSpawnID)
    (bind _asmy_game_instance (Utilities|Casting|CastToMyGameInstance (Game|GetGameInstance)))
    (if (Variables|Default|GetAdd/Remove)
      (Default|Spawn _asmy_game_instance _array_element)
      (else
        (Default|RemoveSpawn _asmy_game_instance _array_element))))
  (Actor|DestroyActor))

(event EventBeginPlay
  ;[1 1 1] Text Visual
  (if (Variables|Default|GetAdd/Remove)
    (Variables|Default|SetChanges (Utilities|String|Append (Variables|Default|GetChanges) "Adds "))
    (else
      (Variables|Default|SetChanges (Utilities|String|Append (Variables|Default|GetChanges) "Removes "))))
  (for _array_element (Variables|Default|GetSpawnID)
    (Variables|Default|SetChanges (Utilities|String|Append (Utilities|String|Append (Variables|Default|GetChanges) (Utilities|String|ToString(Integer) _array_element)) ", ")))
  (Rendering|Components|TextRender|SetText (Variables|Default|GetTextRender) (Utilities|Text|ToText(String) (Variables|Default|GetChanges))))

(fn ConstructionScript)